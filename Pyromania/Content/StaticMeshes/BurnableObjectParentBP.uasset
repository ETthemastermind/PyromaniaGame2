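; Parent Blueprint for burnable objects that the fire character burns and the water character restores by holding E inside the overlap sphere.
; Tick lowers or raises Health through one-second Delays, destroying the actor when burning empties it.
; Exact matches against Health-fifth thresholds computed at BeginPlay toggle and scale the fire effect.
; A world-space widget shows Health as a progress bar and rotates toward the camera.
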(event OnComponentBeginOverlap(Sphere)
  (params (OverlappedComponent :type Primitive%20Component%20Object%20Reference) (OtherActor :type Actor%20Object%20Reference) (OtherComp :type Primitive%20Component%20Object%20Reference) (OtherBodyIndex :type Integer) (bFromSweep :type Boolean) (SweepResult :type Hit%20Result%20Structure%20%28by%20ref%29))
  (Variables|Default|SetOverlapping true))

(event OnComponentEndOverlap(Sphere)
  (params (OverlappedComponent :type Primitive%20Component%20Object%20Reference) (OtherActor :type Actor%20Object%20Reference) (OtherComp :type Primitive%20Component%20Object%20Reference) (OtherBodyIndex :type Integer))
  (Variables|Default|SetOverlapping false))

(event EventTick
  (params (DeltaSeconds :type Float%20%28single-precision%29))
  (bind _fire (Variables|Default|GetFIre))
  (bind _widget (Variables|Default|GetWidget))
  (Utilities|FlowControl|Sequence
    (:then_0
      ;[1 1 1] Checks if the player is playing as "Fire" and will subtract from the item's health
      (bind _asfemale_fire_charcter (Utilities|Casting|CastToFemaleFireCharcter (Game|GetPlayerCharacter 0)))
      (if (Math|Boolean|ANDBoolean (Variables|Default|GetEHeld) (Variables|Default|GetOverlapping) (Variables|/Game/PlayerModels/FemaleFire/FemaleFireCharcter.FemaleFireCharcter_C|GetPlayerFire _asfemale_fire_charcter))
        (Utilities|FlowControl|Delay 1.0)
        (Variables|Default|SetHealth (- (Variables|Default|GetHealth) 1.0))
        (if (<= (Variables|Default|GetHealth) 0.0)
          (Actor|DestroyActor)
          (else
            (Development|PrintString (Utilities|String|ToString(Float) (Variables|Default|GetHealth)))))))
    (:then_1
      ;[1 1 1] Checks if the player is playing as "Water" and will add to the item's health
      (bind _asfemale_water_character (Utilities|Casting|CastToFemaleWaterCharacter (Game|GetPlayerCharacter 0)))
      (if (Math|Boolean|ANDBoolean (Variables|Default|GetEHeld) (Variables|Default|GetOverlapping) (Variables|/Game/PlayerModels/FemaleWater/FemaleWaterCharacter.FemaleWaterCharacter_C|GetPlayerWater _asfemale_water_character))
        (Utilities|FlowControl|Delay 1.0)
        (Variables|Default|SetHealth (+ (Variables|Default|GetHealth) 1.0))
        (Development|PrintString (Utilities|String|ToString(Float) (Variables|Default|GetHealth)))))
    (:then_2
      ;[1 1 1] Controls the size of the fire when the object is on fire
      (if (== (Variables|Default|GetHealth) (Variables|Default|GetFireStage1))
        (Components|Activation|Deactivate _fire))
      (if (== (Variables|Default|GetHealth) (Variables|Default|GetFireStage2))
        (Components|Activation|Activate _fire false)
        (Transformation|SetRelativeScale3D _fire (Variables|Default|GetFireSize1)))
      (if (== (Variables|Default|GetHealth) (Variables|Default|GetFireStage3))
        (Transformation|SetRelativeScale3D _fire (Variables|Default|GetFireSize2)))
      (if (== (Variables|Default|GetHealth) (Variables|Default|GetFireStage4))
        (Transformation|SetRelativeScale3D _fire (Variables|Default|GetFireSize3)))
      (if (== (Variables|Default|GetHealth) (Variables|Default|GetFireStage5))
        (Transformation|SetRelativeScale3D _fire (Variables|Default|GetFireSize4))
        (if (== (Variables|Default|GetHealth) 0.0)
          (Transformation|SetRelativeScale3D _fire (Variables|Default|GetFireSize5)))))
    (:then_3
      ;[1 1 1] Controls the Progress Bar
      (bind _ashealth_bars (Utilities|Casting|CastToHealthBars (UserInterface|GetUserWidgetObject (Variables|Default|GetWidget))))
      (Progress|SetPercent (Variables|/Game/HealthBars.HealthBars_C|GetProgressBar_75 _ashealth_bars) (/ (Variables|Default|GetHealth) (Variables|Default|GetProgressBarModifier)))
      (Transformation|SetWorldRotation _widget (Math|Rotator|FindLookatRotation (Transformation|GetWorldLocation _widget) (Camera|GetCameraLocation (Game|GetPlayerCameraManager 0))) false false))))

(event EventBeginPlay
  (bind _health (Variables|Default|GetHealth))
  (Variables|Default|SetProgressBarModifier (Variables|Default|GetHealth))
  (Variables|Default|SetFireStage1 (* (/ _health 5.0) 5.0))
  (Variables|Default|SetFireStage2 (* (/ _health 5.0) 4.0))
  (Variables|Default|SetFireStage3 (* (/ _health 5.0) 3.0))
  (Variables|Default|SetFireStage4 (* (/ _health 5.0) 2.0))
  (Variables|Default|SetFireStage5 (* (/ _health 5.0) 1.0))
  (Variables|Default|SetFireSize1 (Transformation|GetWorldScale (Variables|Default|GetFIre)))
  (Variables|Default|SetFireSize2 (+ (Variables|Default|GetFireSize1) (Variables|Default|GetFireSize1)))
  (Variables|Default|SetFireSize3 (+ (Variables|Default|GetFireSize2) (Variables|Default|GetFireSize1)))
  (Variables|Default|SetFireSize4 (+ (Variables|Default|GetFireSize3) (Variables|Default|GetFireSize1)))
  (Variables|Default|SetFireSize5 (+ (Variables|Default|GetFireSize4) (Variables|Default|GetFireSize1))))

(event Input|KeyboardEvents|E
  (params (Key :type Key%20Structure :default "AnyKey"))
  (:Pressed
    (Variables|Default|SetEHeld true))
  (:Released
    (Variables|Default|SetEHeld false)))

(fn ConstructionScript)